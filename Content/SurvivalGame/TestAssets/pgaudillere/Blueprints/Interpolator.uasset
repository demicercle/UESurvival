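; Interpolator Blueprint that moves a Target along a spline path, starting automatically on BeginPlay.
; The construction script builds the spline from the local origin, treating each Path entry as an offset from the previous point.
; While started, Tick calls FollowPath with speed, rotation axis and collision settings; on completion it fires Reached and stops.
; StartInterpolation can retarget or reset the position, and an invalid Target halts movement.
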(event `self.ReceiveBeginPlay`
  (`self.StartInterpolation` (`self.Target`)))

(event `StartInterpolation`
  (params (Target :type "Actor Object Reference") (Reset :type Boolean :default true))
  (`/Engine/EditorBlueprintResources/StandardMacros.IsValid` Target
    (:`Is Valid`
      (set `self.Target` Target)
      (set `self.IsStarted` true)
      (if Reset
        (set `self.Position` 0.0)))))

(event `StopInterpolation`
  (set `self.IsStarted` false))

(event `UpdateInterpolation`
  (bind _target (`self.Target`))
  (`/Engine/EditorBlueprintResources/StandardMacros.IsValid` _target
    (:`Is Valid`
      (bind _reached (`/Game/SurvivalGame/Blueprints/Base/Libraries/FunctionLibrary.FollowPath` _target (`self.Spline`) (`self.Position`) (`self.MoveSpeed`) (`self.RotationAxis`) (`self.IgnoreCollisions`)))
      (if _reached
        (`self.Reached`)
        (`self.StopInterpolation`)))
    (:`Is Not Valid`
      (`self.StopInterpolation`))))

(event `self.ReceiveTick`
  (params (DeltaSeconds :type "Float (single-precision)"))
  (if (`self.IsStarted`)
    (`self.UpdateInterpolation`)))

(fn `UserConstructionScript`
  (locals (LastSplinePoint :type "Vector Structure"))
  (bind _spline (`self.Spline`))
  (`SplineComponent.ClearSplinePoints` _spline false)
  (for _array_element (`self.Path`)
    (bind _output_get (set `local.LastSplinePoint` (+ _array_element (stale _output_get))))
    (`SplineComponent.AddSplinePoint` _spline _output_get "Local" false))
  (`SplineComponent.AddSplinePointAtIndex` _spline (`KismetMathLibrary.MakeVector` 0.0) 0 "Local" true))