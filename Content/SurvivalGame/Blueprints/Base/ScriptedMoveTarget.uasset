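; Target actor that drives its owning Pawn to its own location through a scripted AI move.
; On the first Tick with a valid Pawn owner, it spawns an AI controller for that Pawn and runs AIMoveTo toward itself.
; On success or failure it fires the matching dispatcher, spawns the Pawn's default controller, and destroys itself if AutoDestroy is set.
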(event `self.ReceiveBeginPlay`
  (bind _aspawn (cast `Pawn` (`self.GetOwner`)))
  (set `self.Pawn` _aspawn))

(event `self.ReceiveTick`
  (params (DeltaSeconds :type "Float (single-precision)"))
  (bind _pawn (`self.Pawn`))
  (`/Engine/EditorBlueprintResources/StandardMacros.IsValid` _pawn
    (:`Is Valid`
      (if (not (`self.MoveStarted`))
        (set `self.MoveStarted` true)
        (`/Game/SurvivalGame/Blueprints/Base/Libraries/MacroLibrary.SpawnAIController` _pawn)
        (`|AIMoveTo` _pawn (0.0 0.0 0.0) self
          (:`OnSuccess`
            (`self.OnSuccess`))
          (:`OnFail`
            (`self.OnFailed`)))
        (`Pawn.SpawnDefaultController` _pawn)
        (if (`self.AutoDestroy`)
          (`self.K2_DestroyActor` self))))))

(fn `UserConstructionScript`)