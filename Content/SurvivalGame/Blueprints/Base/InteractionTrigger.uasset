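; Base interaction trigger actor that runs a scripted sequence on the instigator when its InteractionComponent fires.
; It disables input, optionally turns the instigator to look at and move to the target, then waits a delay.
; It then runs configured console commands and plays a montage list on Characters, signalling anim start and finish before restoring input.
; The construction script shapes a spline from the component's minimum interaction angle.
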(event `self.InteractionComponent.OnInteracted`
  (params (Instigator :type "Pawn Object Reference"))
  (bind _executeanimations (`self.ExecuteAnimations`))
  (bind (_ascharacter _bsuccess) (cast `Character` (`self.LastInstigator`) :!pure true))
  (`/Engine/EditorBlueprintResources/StandardMacros.IsValid` Instigator
    (:`Is Valid`
      (`/Game/SurvivalGame/Blueprints/Base/Libraries/FunctionLibrary.SetInput` (`self.LastInstigator`) false)
      (if (`self.LookAt`)
        (`/Game/SurvivalGame/Blueprints/Base/Libraries/MacroLibrary.PlayLookAt` (`self.LastInstigator`) (`SceneComponent.K2_GetComponentLocation` (`self.POV`)) (`self.InteractionTarget`) 180.0
          (:`Finished`
            _)))
      (if (`self.MoveTowards`)
        (`/Game/SurvivalGame/Blueprints/Base/Libraries/MacroLibrary.PlayMoveTowards` (`self.LastInstigator`) (`self.InteractionTarget`) (`SceneComponent.K2_GetComponentLocation` (`self.Target`))
          (:`Finished`
            _)))
      (`KismetSystemLibrary.RetriggerableDelay` (`self.ExecuteDelay`))
      (`|ExecutionSequence`
        (:`then_0`
          (`KismetSystemLibrary.PrintString` "Interacted")
          (bind _asplayer_controller (cast `PlayerController` (`Pawn.GetController` (`self.LastInstigator`))))
          (for _array_element (`self.ExecuteCommands`)
            (`KismetSystemLibrary.ExecuteConsoleCommand` _array_element _asplayer_controller)
            (`KismetSystemLibrary.PrintString` _array_element)))
        (:`then_1`
          (if (and (> (`KismetArrayLibrary.Array_Length` _executeanimations) 0) _bsuccess)
            (`/Game/SurvivalGame/Blueprints/Base/Libraries/MacroLibrary.PlayMontageMultiple` _ascharacter _executeanimations
              (:`Started`
                (`self.AnimStarted`)
                (`KismetSystemLibrary.PrintString` "Anim Started"))
              (:`Finished`
                (`self.AnimFinished`)
                (`KismetSystemLibrary.PrintString` "Anim Finished")
                (`/Game/SurvivalGame/Blueprints/Base/Libraries/FunctionLibrary.SetInput` (`self.LastInstigator`) :!label _label)
                (`KismetSystemLibrary.PrintString` "Restore Inputs")))
            (else
              (goto _label))))))))

(fn `UserConstructionScript`
  (locals (SplineTargets :type "Array of Transform Structure"))
  (`/Game/SurvivalGame/Blueprints/Base/Libraries/FunctionLibrary.SetSplineFromAngles` (`self.Spline`) (`/Game/SurvivalGame/Blueprints/Base/Components/InteractionComponent.MinAngle` (`self.InteractionComponent`))))