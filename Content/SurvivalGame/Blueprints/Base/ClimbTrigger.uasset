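; Interactable climb trigger that carries a character straight up to a configurable climb height, like a ladder.
; Interaction makes the character kinematic and plays a looping montage while Tick, enabled only during the climb, moves it upward at constant speed.
; Near the top, a finishing montage plays, and an auto-close gate restores non-kinematic state on the first notify or completion.
; The construction script draws the spline path and adds a capsule at its end.
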(event `self.ReceiveBeginPlay`
  (`self.SetActorTickEnabled` false))

(event `self.InteractionComponent.OnInteracted`
  (params (Instigator :type "Pawn Object Reference"))
  (set `self.LastInstigator` Instigator)
  (`self.StartClimb`))

(event `StartClimb`
  (bind _ascharacter (cast `Character` (`self.LastInstigator`)))
  (`/Game/SurvivalGame/Blueprints/Base/Libraries/FunctionLibrary.SetKinematic` _ascharacter true)
  (`|PlayMontage` (`Character.Mesh` _ascharacter) (`self.LoopMontage`) ; Loop Montage
    (:`then`
      (`self.SetActorTickEnabled` true))))

(event `self.ReceiveTick`
  (params (DeltaSeconds :type "Float (single-precision)"))
  (bind _lastinstigator (`self.LastInstigator`))
  (bind _returnvalue (`self.K2_GetActorLocation` _lastinstigator))
  (bind _returnvalue_2 (`KismetMathLibrary.TransformLocation` (`self.GetTransform`) (`KismetMathLibrary.MakeVector` 0.0 0.0 (`self.ClimbHeight`))))
  (`/Engine/EditorBlueprintResources/StandardMacros.IsValid` (`self.LastInstigator`)
    (:`Is Valid`
      (`self.K2_SetActorLocation` _lastinstigator (`KismetMathLibrary.VInterpTo_Constant` _returnvalue _returnvalue_2 DeltaSeconds 100.0) false false)
      (if (<= (`KismetMathLibrary.Vector_Distance` _returnvalue _returnvalue_2) 5.0)
        (`self.StopClimb`)))))

(event `StopClimb`
  (bind _ascharacter (cast `Character` (`self.LastInstigator`)))
  (`|PlayMontage` (`Character.Mesh` _ascharacter) (`self.TopMontage`)
    (:`then`
      (`|ExecutionSequence`
        (:`then_0`
          (`self.SetActorTickEnabled` false))
        (:`then_1`
          (goto _label :!via `Open`))))
    (:`OnCompleted`
      (`/Game/SurvivalGame/Blueprints/Base/Libraries/MacroLibrary.AutoCloseGate` true :!label _label
        (:`Exit`
          (`/Game/SurvivalGame/Blueprints/Base/Libraries/FunctionLibrary.SetKinematic` (`self.LastInstigator`)))))
    (:`OnNotifyBegin`
      (goto _label))))

(fn `UserConstructionScript`
  (bind _spline (`self.Spline`))
  (bind _returnvalue (`KismetMathLibrary.MakeVector` 0.0 0.0 (`self.ClimbHeight`)))
  (bind _returnvalue_2 (+ _returnvalue (0.0 0.0 92.0)))
  (bind _returnvalue_3 (+ _returnvalue_2 (-45.0 0.0 92.0)))
  (`/Game/SurvivalGame/Blueprints/Base/Libraries/EditorFunctionLibrary.ConstructMoveTarget` (`self.MoveTargetComponent`))
  (`/Game/SurvivalGame/Blueprints/Base/Libraries/EditorFunctionLibrary.ConstructInteractionComponent` (`self.InteractionComponent`))
  (`SplineComponent.SetSplinePoints` (`self.Spline`) (`|MakeArray` (0.0 0.0 0.0) _returnvalue _returnvalue_2 _returnvalue_3) "Local" true)
  (`/Game/SurvivalGame/Blueprints/Base/Libraries/FunctionLibrary.DestroyAllComponents` _spline)
  (bind _returnvalue_4 (`AddComponent|NODE_AddCapsuleComponent-0` :`bManualAttachment` true))
  (`SceneComponent.K2_AttachToComponent` _returnvalue_4 _spline "None" "SnapToTarget" "SnapToTarget" "SnapToTarget" true)
  (`SceneComponent.K2_SetRelativeLocation` _returnvalue_4 _returnvalue_3 false false)
  (`CapsuleComponent.SetCapsuleSize` _returnvalue_4 45.0 92.0 true))