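; Base interaction component for actors in a survival game, started by an event that receives the instigator.
; With LookAt and MoveTowards off, it waits out a retriggerable delay, broadcasts OnInteracted and runs configured console commands on the first player controller.
; It marks itself finished unless animations exist for a Character instigator, but animation playback and its callbacks are unwired.
; RequestInteraction and UpdateInteraction are stubs returning false.
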(event `/Game/SurvivalGame/Blueprints/Base/Interfaces/IInteractable.StartInteraction`
  (params (Instigator :type "Pawn Object Reference"))
  (bind _returnvalue (and (> (`KismetArrayLibrary.Array_Length` (`self.Animations`)) 0) (`.bSuccess` (cast `Character` Instigator :!pure true))))
  (set `self.Finished` false)
  (`/Engine/EditorBlueprintResources/StandardMacros.IsValid` Instigator
    (:`Is Valid`
      (if (`self.LookAt`)
        _
        (elif (not (`self.MoveTowards`))
          (`KismetSystemLibrary.RetriggerableDelay` (`self.InteractionDelay`))
          (`self.OnInteracted`)
          (`|ExecutionSequence`
            (:`then_0`
              (set `self.Finished` (not _returnvalue))
              (for _array_element (`self.ExecuteCommands`)
                (`KismetSystemLibrary.ExecuteConsoleCommand` _array_element (`GameplayStatics.GetPlayerController` 0))))
            (:`then_1`
              (if _returnvalue
                _))))))))

(fn `RequestInteraction`
  (params (Instigator :type "Pawn Object Reference"))
  (returns (Success :type Boolean))
  (return false))

(fn `UpdateInteraction`
  (params (Instigator :type "Pawn Object Reference"))
  (returns (Finished :type Boolean))
  (return false))