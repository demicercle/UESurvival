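; Patrol waypoint actor that routes pawns through a branching network of linked points.
; When reached, it waits a random duration, then turns Characters to its facing and plays a random montage with input disabled, if any are configured.
; It then sends the pawn to a random NextPoints entry via ScriptedPatrol.
; Its construction script makes every PatrolPoint in the level rebuild blue arrow components visualizing its outgoing links.
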(event `Reached_Event`
  (params (Pawn :type "Pawn Object Reference"))
  (bind _animations (`self.Animations`))
  (bind _lastpawnreach (`self.LastPawnReach`))
  (bind (_lowerbound _upperbound) (break `FloatRange` (`self.WaitDuration`)))
  (bind _returnvalue (`KismetArrayLibrary.Array_Length` _animations))
  (bind (_montage _playrate _starttime _maxloop) (break `/Game/SurvivalGame/Blueprints/Base/Structs/AnimationParams` (`|GetArrayItem` _animations (`KismetMathLibrary.RandomIntegerInRange` 0 (- _returnvalue 1)))))
  (set `self.LastPawnReach` Pawn)
  (`KismetSystemLibrary.Delay` (`KismetMathLibrary.RandomFloatInRange` (`.Value` (break `FloatRangeBound` _lowerbound)) (`.Value` (break `FloatRangeBound` _upperbound))))
  (if (> _returnvalue 0)
    (bind _ascharacter (cast `Character` _lastpawnreach)
      (:`then`
        (`/Game/SurvivalGame/Blueprints/Base/Libraries/FunctionLibrary.SetInputEnabled` _lastpawnreach false)
        (`/Game/SurvivalGame/Blueprints/Base/Libraries/MacroLibrary.PlayRotateTowards` _ascharacter (`self.K2_GetActorRotation`) 180.0 1.0 false
          (:`Finished`
            (`/Game/SurvivalGame/Blueprints/Base/Libraries/MacroLibrary.PlayMontage` _ascharacter _montage _playrate _starttime _maxloop
              (:`Finished`
                (`/Game/SurvivalGame/Blueprints/Base/Libraries/FunctionLibrary.SetInputEnabled` (`self.LastPawnReach`)))))))
      (:`CastFailed`
        _)))
  (bind (_success _output) (`self.GetNextPoint`))
  (if _success
    (`/Game/SurvivalGame/Blueprints/Base/Libraries/MacroLibrary.ScriptedPatrol` (`self.LastPawnReach`) _output)))

(fn `GetNextPoint`
  (returns (Success :type Boolean) (Output :type "/Game/SurvivalGame/Blueprints/Base/PatrolPoint Object Reference"))
  (bind _nextpoints (`self.NextPoints`))
  (bind _output (`|GetArrayItem` _nextpoints (`KismetMathLibrary.RandomIntegerInRange` 0 (- (`KismetArrayLibrary.Array_Length` _nextpoints) 1))))
  (return (`KismetSystemLibrary.IsValid` _output) _output))

(fn `UpdateConnections`
  (bind _returnvalue (`self.K2_GetActorLocation`))
  (for _array_element (`SceneComponent.GetChildrenComponents` (`self.Scene`) false)
    (`ActorComponent.K2_DestroyComponent` _array_element))
  (for _array_element_2 (`self.NextPoints`)
    (`/Engine/EditorBlueprintResources/StandardMacros.IsValid` _array_element_2
      (:`Is Valid`
        (bind _returnvalue_2 (`AddComponent|NODE_AddArrowComponent-0` :`bManualAttachment` true :`RelativeTransform` (`KismetMathLibrary.MakeTransform` (0.0 0.0 0.0))))
        (`SceneComponent.K2_AttachToComponent` _returnvalue_2 (`self.Scene`) "None" "SnapToTarget" "SnapToTarget" "SnapToTarget" true)
        (bind _returnvalue_3 (`self.K2_GetActorLocation` _array_element_2))
        (set `ArrowComponent.ArrowLength` (- (`KismetMathLibrary.Vector_Distance` _returnvalue _returnvalue_3) 20.0) _returnvalue_2)
        (set `ArrowComponent.ArrowSize` 1.0 _returnvalue_2)
        (`ArrowComponent.SetArrowColor` _returnvalue_2 (struct :`G` 0.146584 :`B` 1.0 :`A` 1.0))
        (`SceneComponent.K2_SetWorldRotation` _returnvalue_2 (`KismetMathLibrary.MakeRotFromX` (- _returnvalue_3 _returnvalue)) false false)))))

(fn `UserConstructionScript`
  (bind _outactors (`GameplayStatics.GetAllActorsOfClass` "PatrolPoint_C"))
  (for _array_element _outactors
    (`self.UpdateConnections` _array_element)))