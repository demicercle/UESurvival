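; Blueprint function library of shared helpers for debug output, actor movement, montage playback and recursive attached-actor lookup.
; DebugPrint writes to the first DebugHUD widget, while RotateActor and MoveActor interpolate per call and report arrival.
; TryPlayAnimation starts montages up to a loop limit, tracked in a by-ref counter.
; FollowPath advances a by-ref spline distance through SetLocationAndRotation, which also sets Pawn control rotation and can temporarily disable collision.
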(fn `DebugPrint`
  (params (Text :type String) (Prepend :type String) (Append :type String) (NewLine :type Boolean :default true))
  (bind _foundwidgets (`WidgetBlueprintLibrary.GetAllWidgetsOfClass` null "/Game/SurvivalGame/HUD/DebugHUD.DebugHUD_C"))
  (if (> (`KismetArrayLibrary.Array_Length` _foundwidgets) 0)
    (`/Game/SurvivalGame/HUD/DebugHUD.Print` (`|GetArrayItem` _foundwidgets) (`KismetStringLibrary.Concat_StrStr` Prepend " " Text " " Append) NewLine)))

(fn `FollowPath`
  (params (Target :type "Actor Object Reference") (Spline :type "SplineComponent Object Reference (by ref)") (Position :type "Float (double-precision) (by ref)") (MoveSpeed :type "Float (double-precision)") (RotationAxis :type "Vector Structure" :default (1.0 1.0 1.0)) (IgnoreCollisions :type Boolean))
  (returns (Reached :type Boolean))
  (bind _returnvalue (`SplineComponent.GetSplineLength` Spline))
  (bind _returnvalue_2 (`KismetMathLibrary.SelectFloat` (/ Position _returnvalue) 1.0 (> _returnvalue 0.0)))
  (`self.SetLocationAndRotation` Target (`SplineComponent.GetLocationAtTime` Spline _returnvalue_2 "Local" false) (`KismetMathLibrary.MakeRotator` (* (.roll (`SplineComponent.GetRotationAtTime` Spline _returnvalue_2 "Local" false)) (.x RotationAxis)) (* (.pitch (`SplineComponent.GetRotationAtTime` Spline _returnvalue_2 "Local" false)) (.y RotationAxis)) (* (.yaw (`SplineComponent.GetRotationAtTime` Spline _returnvalue_2 "Local" false)) (.z RotationAxis))) IgnoreCollisions)
  (if (>= Position _returnvalue)
    (return true)
    (else
      (`|VariableSetRef` Position (+ Position (* MoveSpeed (`GameplayStatics.GetWorldDeltaSeconds` null)))))))

(fn `GetAttachedActorsRecursive`
  (params (Target :type "Actor Object Reference"))
  (returns (OutActors :type "Array of Actor Object Reference"))
  (locals (Output :type "Array of Actor Object Reference"))
  (bind _output_get (set `local.Output` (`Actor.GetAttachedActors` Target true)))
  (for _array_element _output_get
    (bind _outactors (`self.GetAttachedActorsRecursive` _array_element))
    (for _array_element_2 _outactors
      (`KismetArrayLibrary.Array_Add` (`local.Output`) _array_element_2)))
  (return (`local.Output`)))

(fn `MoveActor`
  (params (Actor :type "Actor Object Reference") (Location :type "Vector Structure") (MinDistance :type "Float (double-precision)" :default 10.0) (Speed :type "Float (double-precision)" :default 100.0) (DeltaTime :type "Float (double-precision)"))
  (returns (Reached :type Boolean))
  (bind _returnvalue (`Actor.K2_GetActorLocation` Actor))
  (`Actor.K2_SetActorLocation` Actor (`KismetMathLibrary.VInterpTo_Constant` _returnvalue Location DeltaTime Speed) false false)
  (return (<= (`KismetMathLibrary.Vector_Distance` _returnvalue Location) MinDistance)))

(fn `RotateActor`
  (params (Actor :type "Actor Object Reference") (Rotation :type "Rotator Structure") (MinAngle :type "Float (double-precision)" :default 10.0) (Speed :type "Float (double-precision)" :default 180.0) (DeltaTime :type "Float (double-precision)"))
  (returns (Reached :type Boolean))
  (bind _aspawn (cast `Pawn` Actor))
  (bind _returnvalue (`Pawn.GetController` _aspawn))
  (bind _returnvalue_2 (`Controller.GetControlRotation` _returnvalue))
  (`Controller.SetControlRotation` _returnvalue (`KismetMathLibrary.RInterpTo_Constant` _returnvalue_2 Rotation DeltaTime Speed))
  (return (<= (.yaw (`KismetMathLibrary.NormalizedDeltaRotator` _returnvalue_2 Rotation)) MinAngle)))

(fn `SetLocationAndRotation`
  (params (Target :type "Actor Object Reference") (Location :type "Vector Structure" :default (0.0 0.0 1.0)) (Rotation :type "Rotator Structure") (IgnoreCollisions :type Boolean))
  (locals (RestoreCollision :type Boolean))
  (`|ExecutionSequence`
    (:`then_0`
      (bind _aspawn (cast `Pawn` Target))
      (`Controller.SetControlRotation` (`Pawn.GetController` _aspawn) Rotation))
    (:`then_1`
      (if IgnoreCollisions
        (set `local.RestoreCollision` (`Actor.GetActorEnableCollision` Target))
        (`Actor.SetActorEnableCollision` Target false))
      (`Actor.K2_SetActorLocationAndRotation` Target Location Rotation false false)
      (if IgnoreCollisions
        (`Actor.SetActorEnableCollision` Target (`local.RestoreCollision`)))
      (return))))

(fn `TryPlayAnimation`
  (params (Actor :type "Actor Object Reference") (Montage :type "AnimMontage Object Reference") (PlayRate :type "Float (double-precision)" :default 1.0) (StartTime :type "Float (double-precision)") (StopOthers :type Boolean :default true) (MaxLoop :type Integer :default 0) (LoopCount :type "Integer (by ref)"))
  (returns (Played :type Boolean) (Started :type Boolean) (Finished :type Boolean) (Duration :type "Float (double-precision)"))
  (bind _returnvalue (/ (`AnimSequenceBase.SequenceLength` Montage) PlayRate))
  (`/Engine/EditorBlueprintResources/StandardMacros.IsValid` Montage
    (:`Is Valid`
      (bind _ascharacter (cast `Character` Actor)
        (:`then`
          (bind _returnvalue_2 (`SkeletalMeshComponent.GetAnimInstance` (`Character.Mesh` _ascharacter)))
          (if (`AnimInstance.Montage_IsPlaying` _returnvalue_2 Montage)
            (return true false false _returnvalue)
            (elif (<= LoopCount MaxLoop)
              (`|VariableSetRef` LoopCount (+ LoopCount 1))
              (bind _returnvalue_3 (`AnimInstance.Montage_Play` _returnvalue_2 Montage PlayRate "MontageLength" StartTime StopOthers))
              (return true true false _returnvalue_3)
              (else
                _))))
        (:`CastFailed`
          _)))
    (:`Is Not Valid`
      _))
  (return false false true _returnvalue))