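; Interactable actor that carries an instigator along a spline while playing montages timed to points on the path.
; The construction script builds the spline from relative Path offsets, marking animation starts with billboards and adding a capsule at the end.
; RequestInteraction gates on yaw and availability.
; UpdateInteraction advances time by speed, moves the instigator only when IgnoreCollision is set, and reports completion once the path and non-looping montages are done.
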(event `/Game/SurvivalGame/Blueprints/Interfaces/IInteractable.StartInteraction`
  (`self.Interacted`))

(fn `Attach Component to Spline`
  (params (Time :type "Float (double-precision)") (Component :type "ActorComponent Object Reference"))
  (returns (ReturnValue :type "ActorComponent Object Reference"))
  (bind _returnvalue (`|AddComponentByClass` (`GameplayStatics.GetObjectClass` Component)))
  (bind _asscene_component (cast `SceneComponent` _returnvalue)
    (:`then`
      (`SceneComponent.K2_SetRelativeLocation` _asscene_component (`SplineComponent.GetLocationAtTime` (`self.Spline`) (`KismetMathLibrary.FClamp` Time) "Local" false) false false)
      (`SceneComponent.SetVisibility` _asscene_component true false)
      (`SceneComponent.K2_AttachToComponent` _asscene_component (`self.Spline`) "None" "KeepRelative" "KeepRelative" "KeepRelative" true))
    (:`CastFailed`
      _))
  (return _returnvalue))

(fn `RequestInteraction`
  (params (Instigator :type "Pawn Object Reference"))
  (returns (Success :type Boolean))
  (return (and (<= (.yaw (`KismetMathLibrary.NormalizedDeltaRotator` (`self.K2_GetActorRotation` Instigator) (`self.K2_GetActorRotation`))) (`self.InteractionAngle`)) (`self.CanBeInteracted`))))

(fn `UpdateInteraction`
  (params (Instigator :type "Pawn Object Reference"))
  (returns (Finished :type Boolean))
  (bind _spline (`self.Spline`))
  (bind _returnvalue (`SplineComponent.GetSplineLength` (`self.Spline`)))
  (bind _returnvalue_2 (`SplineComponent.GetNumberOfSplinePoints` _spline))
  (bind _returnvalue_3 (`SplineComponent.GetLocationAtTime` (`self.Spline`) (`self.SplineTime`) "World" false))
  (`|ExecutionSequence`
    (:`then_0`
      ;[1 1 1] Started
      (if (not (`self.Started`))
        (set `self.Started` true)
        (`KismetArrayLibrary.Array_Clear` (`self.PlayedAnimations`))
        (set `self.SplinePosition` 0.0)
        (set `self.MinPlayedAnimations` 0)
        (for _array_element (`self.Animations`)
          (if (not (`.Loop_29_E2D58D5D445AE36B151929AA82C0E86C` (break `/Game/SurvivalGame/TestAssets/pgaudillere/SplineAnimation` _array_element)))
            (`/Engine/EditorBlueprintResources/StandardMacros.IncrementInt` (`self.MinPlayedAnimations`)))))
      ;[1 1 1] Set Time
      (set `self.SplineTime` (`KismetMathLibrary.SelectFloat` 1.0 (/ (`self.SplinePosition`) _returnvalue) (== _returnvalue 0.0)))
      ;[1 1 1] Update Position
      (bind _output_get (set `self.SplinePosition` (+ (stale _output_get) (* (`GameplayStatics.GetWorldDeltaSeconds`) (`self.MoveSpeed`))))))
    (:`then_1`
      ;[1 1 1] Update Position & Rotation
      (if (`self.IgnoreCollision`)
        (`self.SetActorEnableCollision` false)
        (`self.K2_SetActorLocationAndRotation` Instigator _returnvalue_3 (`KismetMathLibrary.MakeRotator` 0.0 0.0 (.yaw (`KismetMathLibrary.MakeRotFromX` (- _returnvalue_3 (`SplineComponent.GetLocationAtSplinePoint` _spline (`KismetMathLibrary.Clamp` (`KismetMathLibrary.FCeil` (* _returnvalue_2 (`self.SplineTime`))) 0 (- _returnvalue_2 1)) "World"))))) false false)
        (if (`self.IgnoreCollision`)
          (`self.SetActorEnableCollision` true))))
    (:`then_2`
      ;[1 1 1] Update Animations
      (for _array_element_2 (`self.Animations`)
        (bind (_starttime _montage _playrate _loop) (break `/Game/SurvivalGame/TestAssets/pgaudillere/SplineAnimation` _array_element_2))
        (`/Engine/EditorBlueprintResources/StandardMacros.IsValid` _montage
          (:`Is Valid`
            (if (>= (`self.SplineTime`) _starttime)
              (if (or _loop (not (`KismetArrayLibrary.Array_Contains` (`self.PlayedAnimations`) _montage)))
                (bind (_played _duration _time _playing) (`/Game/SurvivalGame/Blueprints/Libraries/FunctionLibrary.Play Animation` Instigator _montage _playrate))
                (if _playing
                  (`KismetArrayLibrary.Array_AddUnique` (`self.PlayedAnimations`) _montage))))))))
    (:`then_3`
      (if (and (>= (`self.SplineTime`) 1.0) (>= (`KismetArrayLibrary.Array_Length` (`self.PlayedAnimations`)) (`self.MinPlayedAnimations`)))
        (set `self.Started` false)
        (return true)))))

(fn `UpdateSpline`
  (locals (LastSplinePoint :type "Vector Structure"))
  (bind _spline (`self.Spline`))
  ;[1 1 1] Update Points
  (`SplineComponent.ClearSplinePoints` _spline false)
  (for (_array_element _array_index) (`self.Path`)
    (bind _output_get (set `local.LastSplinePoint` (+ _array_element (stale _output_get))))
    (`SplineComponent.AddSplinePointAtIndex` _spline _output_get _array_index "Local" false))
  (`SplineComponent.AddSplinePointAtIndex` _spline (`KismetMathLibrary.MakeVector` 0.0) 0 "Local" true))

(fn `UserConstructionScript`
  (locals (SplineTargets :type "Array of Transform Structure"))
  (bind _animations (`self.Animations`))
  (for _array_element (`SceneComponent.GetChildrenComponents` (`self.Spline`) false)
    (`ActorComponent.K2_DestroyComponent` _array_element))
  (`self.UpdateSpline`)
  ;[1 1 1] Render Animations
  (for (_array_element_2 _array_index) _animations
    (bind (_starttime _montage _playrate _loop) (break `/Game/SurvivalGame/TestAssets/pgaudillere/SplineAnimation` _array_element_2))
    (`KismetArrayLibrary.Array_Set` _animations _array_index (make `/Game/SurvivalGame/TestAssets/pgaudillere/SplineAnimation` (`KismetMathLibrary.FClamp` _starttime) _montage _playrate _loop))
    (`self.Attach Component to Spline` _starttime (`self.Billboard`)))
  (bind _returnvalue (`self.Attach Component to Spline` 1.0 (`self.CollisionComponent`)))
  (bind _ascapsule_collision (cast `CapsuleComponent` _returnvalue))
  (`CapsuleComponent.SetCapsuleSize` _ascapsule_collision 42.0 96.0 true))