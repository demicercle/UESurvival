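; ClimbTarget is an interactable climb point that moves an actor up onto a ledge.
; Construction previews the climb with an up-then-forward spline and matching entry and exit capsules derived from ClimbHeight.
; RequestInteraction optionally runs the player's ClimbCheck to refresh location, rotation and height.
; UpdateInteraction rotates the instigator, plays a 1m or 2m montage chosen by height, disables its collision and moves it to ClimbLocation.
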(fn `RequestInteraction`
  (params (Instigator :type "Pawn Object Reference"))
  (returns (Success :type Boolean))
  (bind _asplayer_character (cast `/Game/SurvivalGame/Blueprints/PlayerCharacter` Instigator))
  (if (`self.NeedClimbCheck`)
    (bind (_result _climblocation _climbrotation _climbheight) (`/Game/SurvivalGame/Blueprints/PlayerCharacter.ClimbCheck` _asplayer_character (`CharacterMovementComponent.MaxStepHeight` (`Character.CharacterMovement` _asplayer_character)) 200.0))
    (set `self.ClimbLocation` _climblocation)
    (set `self.ClimbRotation` _climbrotation)
    (set `self.ClimbHeight` _climbheight)
    (return _result)
    (else
      (return true))))

(fn `UpdateInteraction`
  (params (Instigator :type "Pawn Object Reference"))
  (returns (Finished :type Boolean))
  (bind _reached (`/Game/SurvivalGame/Blueprints/Libraries/FunctionLibrary.RotateActor` Instigator (`self.ClimbRotation`) 10.0 180.0 (`GameplayStatics.GetWorldDeltaSeconds`)))
  (if _reached
    (`/Game/SurvivalGame/Blueprints/Libraries/FunctionLibrary.Play Animation` Instigator (select `int` (`KismetMathLibrary.FFloor` (/ (`self.ClimbHeight`) 100.0)) :`0` "/Game/AnimsetPro/Montages/Climb1m_Montage.Climb1m_Montage" :`1` "/Game/AnimsetPro/Montages/Climb2m_Montage.Climb2m_Montage" :!type "AnimMontage Object Reference"))
    (`self.SetActorEnableCollision` Instigator false)
    (bind _reached_2 (`/Game/SurvivalGame/Blueprints/Libraries/FunctionLibrary.MoveActor` Instigator (`self.ClimbLocation`) 10.0 100.0 (`GameplayStatics.GetWorldDeltaSeconds`)))
    (`self.SetActorEnableCollision` _reached_2)
    (return _reached_2)))

(fn `UserConstructionScript`
  (bind _returnvalue (`self.GetTransform`))
  (bind _spline (`self.Spline`))
  (bind _climblocation (`self.ClimbLocation`))
  (bind _capsulein (`self.CapsuleIn`))
  (bind _capsuleout (`self.CapsuleOut`))
  (bind _location (.location _returnvalue))
  (bind _array (`|MakeArray` _location (`KismetMathLibrary.MakeVector` (.x _location) (.y _location) (.z _climblocation)) _climblocation))
  (set `self.ClimbLocation` (`KismetMathLibrary.TransformLocation` _returnvalue (`KismetMathLibrary.MakeVector` (* (`CapsuleComponent.CapsuleRadius` (`self.CapsuleIn`)) 2.0) 0.0 (`self.ClimbHeight`))))
  (`SplineComponent.SetSplinePoints` _spline _array "World" true)
  (for (_ _array_index) _array
    (`SplineComponent.SetTangentAtSplinePoint` _spline _array_index (`KismetMathLibrary.MakeVector` 0.0) "Local" true)
    (`SceneComponent.K2_SetRelativeRotation` (`self.CapsuleIn`) (`self.ClimbRotation`) false false)
    (`SceneComponent.K2_SetWorldLocation` _capsuleout (`self.ClimbLocation`) false false)
    (`CapsuleComponent.SetCapsuleHalfHeight` _capsuleout (`CapsuleComponent.CapsuleHalfHeight` _capsulein) true)
    (`CapsuleComponent.SetCapsuleRadius` _capsuleout (`CapsuleComponent.GetScaledCapsuleRadius` _capsulein) true)))