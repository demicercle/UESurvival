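; Interaction trigger, named as an old version, that lines an instigator up with its own transform and plays an animation montage.
; RequestInteraction checks that interaction is allowed and the signed yaw difference to the instigator is within the angle limit.
; UpdateInteraction rotates and moves the instigator onto the trigger, then plays the montage with a loop limit and reports completion.
; StartInteraction resets the loop count and fires OnInteracted after a retriggerable delay.
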(event `/Game/SurvivalGame/Blueprints/Interfaces/IInteractable.StartInteraction`
  (set `self.LoopCount` 0)
  (`KismetSystemLibrary.RetriggerableDelay` (`self.InteractionDelay`))
  (`self.OnInteracted`))

(fn `RequestInteraction`
  (params (Instigator :type "Pawn Object Reference"))
  (returns (Success :type Boolean))
  (bind _returnvalue (and (<= (.yaw (`KismetMathLibrary.NormalizedDeltaRotator` (`self.K2_GetActorRotation` Instigator) (`self.K2_GetActorRotation`))) (`self.InteractionAngle`)) (`self.CanBeInteracted`)))
  (if _returnvalue
    (return _returnvalue)))

(fn `UpdateInteraction`
  (params (Instigator :type "Pawn Object Reference"))
  (returns (Finished :type Boolean))
  (bind _returnvalue (`GameplayStatics.GetWorldDeltaSeconds`))
  (bind _reached (`/Game/SurvivalGame/Blueprints/Libraries/FunctionLibrary.RotateActor` Instigator (`self.K2_GetActorRotation`) 0.0 180.0 _returnvalue))
  (bind _reached_2 (`/Game/SurvivalGame/Blueprints/Libraries/FunctionLibrary.MoveActor` Instigator (`self.K2_GetActorLocation`) 10.0 100.0 _returnvalue))
  (if (and _reached _reached_2)
    (bind (_played _started _finished) (`/Game/SurvivalGame/Blueprints/Libraries/FunctionLibrary.TryPlayAnimation` Instigator (`self.AnimMontage`) 1.0 0.0 true (`self.MaxLoop`) (`self.LoopCount`)))
    (return _finished)))

(fn `UserConstructionScript`
  (locals (SplineTargets :type "Array of Transform Structure")))