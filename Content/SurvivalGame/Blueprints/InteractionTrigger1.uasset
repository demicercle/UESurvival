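; An interaction trigger actor that aligns an instigator to a trigger component and plays an animation montage on it.
; Requests pass when the signed yaw difference is within InteractionAngle and CanBeInteracted is set.
; Each update rotates, then moves the instigator, then plays the montage, reporting completion once its duration has elapsed.
; OnInteracted calls Interacted, and the construction script draws a local spline from the origin to LocationOffset.
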(event `/Game/SurvivalGame/Blueprints/Interfaces/IInteractable.OnInteracted`
  (params (Instigator :type "Pawn Object Reference"))
  (`self.Interacted`))

(fn `RequestInteraction`
  (params (Instigator :type "Pawn Object Reference"))
  (returns (Success :type Boolean))
  (return (and (<= (.yaw (`KismetMathLibrary.NormalizedDeltaRotator` (`self.K2_GetActorRotation` Instigator) (`SceneComponent.K2_GetComponentRotation` (`self.Trigger`)))) (`self.InteractionAngle`)) (`self.CanBeInteracted`))))

(fn `UpdateInteraction`
  (params (Instigator :type "Pawn Object Reference"))
  (returns (Finished :type Boolean))
  (bind _returnvalue (`GameplayStatics.GetTimeSeconds`))
  (bind _trigger (`self.Trigger`))
  (bind _reached (`/Game/SurvivalGame/Blueprints/Libraries/FunctionLibrary.RotateActorTowards` Instigator (`SceneComponent.K2_GetComponentRotation` _trigger) 10.0 180.0 (`GameplayStatics.GetWorldDeltaSeconds`)))
  (if _reached
    (bind _reached_2 (`/Game/SurvivalGame/Blueprints/Libraries/FunctionLibrary.MoveActorTowards` Instigator (`SceneComponent.K2_GetComponentLocation` _trigger) 96.0 100.0 (`GameplayStatics.GetWorldDeltaSeconds`)))
    (if _reached_2
      (bind (_playing _duration) (`/Game/SurvivalGame/Blueprints/Libraries/FunctionLibrary.Play Animation` Instigator (`self.AnimMontage`) (`self.AnimPlayRate`) (`self.AnimStartTime`)))
      (if _playing
        (bind _output_get (set `self.LastInteractionTime` (`KismetMathLibrary.SelectFloat` (stale _output_get) _returnvalue (> (stale _output_get) 0.0))))
        (return (>= (- _returnvalue (`self.LastInteractionTime`)) _duration))))))

(fn `UserConstructionScript`
  (`SplineComponent.SetSplinePoints` (`self.Spline`) (`|MakeArray` (0.0 0.0 0.0) (`self.LocationOffset`)) "Local" true))