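; InteractionTarget is an interaction point that aligns an instigating actor to its own transform and plays a montage on it.
; UpdateAnimation sets the instigator's collision from IgnoreCollision, then moves and rotates it by frame delta time.
; The montage starts once aligned, or immediately with AutoStart.
; A stored timestamp tracks montage duration; when playback ends or fails and alignment holds, it calls SetActorEnableCollision(true) and returns false.
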(fn `UpdateAnimation`
  (params (Instigator :type "Pawn Object Reference"))
  (returns (Finished :type Boolean))
  (locals (DeltaTime :type "Float (double-precision)") (Duration :type Boolean))
  (bind _returnvalue (`GameplayStatics.GetTimeSeconds`))
  (`self.SetActorEnableCollision` Instigator (not (`self.IgnoreCollision`)))
  (set `local.DeltaTime` (`GameplayStatics.GetWorldDeltaSeconds`))
  (bind _reached (`/Game/SurvivalGame/Blueprints/Libraries/FunctionLibrary.MoveActor` Instigator (`self.K2_GetActorLocation`) 10.0 (`self.MoveSpeed`) (`local.DeltaTime`)))
  (bind _reached_2 (`/Game/SurvivalGame/Blueprints/Libraries/FunctionLibrary.RotateActor` Instigator (`self.K2_GetActorRotation`) 10.0 (`self.RotationSpeed`) (`local.DeltaTime`)))
  (bind _returnvalue_2 (and _reached _reached_2))
  (if (or _returnvalue_2 (`self.AutoStart`))
    (bind (_played _started _finished _duration _playing _position) (`/Game/SurvivalGame/Blueprints/Libraries/FunctionLibrary.TryPlayAnimation` Instigator (`self.Montage`) (`self.PlayRate`) (`self.StartTime`)))
    (if _playing
      (if (> (`self.LastPlayTime`) 0.0)
        (if (>= (- _returnvalue (`self.LastPlayTime`)) _duration)
          (set `self.LastPlayTime` 0.0)
          (if _returnvalue_2 :!label _label
            (`self.SetActorEnableCollision` true)
            (return false)))
        (else
          (set `self.LastPlayTime` _returnvalue)
          (`KismetSystemLibrary.PrintString` "start montage")))
      (else
        (goto _label)))))

(fn `UserConstructionScript`)